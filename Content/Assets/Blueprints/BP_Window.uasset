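; BP_Window is a window actor whose construction script picks one of several window looks from its material.
; It creates a dynamic material instance on WindowMesh and sets the Offset X and Offset Y parameters to random steps of one third, apparently selecting a cell in a 3x3 layout.
; A seeded random stream drives both picks, with the seed shifted by a random amount before the Y pick.
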(fn `UserConstructionScript`
  (bind _random_stream (`self.Random Stream`))
  (bind _random_seed (`self.Random Seed`))
  (bind _returnvalue (`KismetMathLibrary.FFloor` (`KismetMathLibrary.RandomFloatInRangeFromStream` 0.0 2.99 _random_stream)))
  ;[1 1 1] Window Material setup to allow for switching between the different windnow types on the material
  (`KismetMathLibrary.SetRandomStreamSeed` _random_stream _random_seed)
  (bind _returnvalue_2 (`PrimitiveComponent.CreateDynamicMaterialInstance` (`self.Window Mesh`) 0 null))
  (`MaterialInstanceDynamic.SetScalarParameterValue` _returnvalue_2 "Offset X" (/ (`KismetMathLibrary.Conv_IntToDouble` _returnvalue) 3.0))
  (`KismetMathLibrary.SetRandomStreamSeed` _random_stream (+ _random_seed _returnvalue))
  (`MaterialInstanceDynamic.SetScalarParameterValue` _returnvalue_2 "Offset Y" (/ (`KismetMathLibrary.Conv_IntToDouble` (`KismetMathLibrary.FFloor` (`KismetMathLibrary.RandomFloatInRangeFromStream` 0.0 2.99 _random_stream))) 3.0)))