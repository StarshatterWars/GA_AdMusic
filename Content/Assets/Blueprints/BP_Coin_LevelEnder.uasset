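; BP_Coin_LevelEnder is a level-ending coin that sends the player to the level selected by NextLevel.
; Sphere overlap, with no actor filter, clears the coin mesh, disables character input and temporarily blocks level skipping.
; After a short delay it calls the matching MyCharacter move function; mesh and level skip return later.
; The construction script applies CoinMaterial; DestroyActor is unwired, so the coin persists.
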(event `self.SphereTrigger.OnComponentBeginOverlap`
  (params (OtherActor :type "Actor Object Reference") (OtherComp :type "PrimitiveComponent Object Reference") (OtherBodyIndex :type Integer) (bFromSweep :type Boolean) (SweepResult :type "EngineTypes.HitResult Structure (by ref)"))
  (bind _coin (`self.Coin`))
  (`|ExecutionSequence`
    (:`then_0`
      ;[1 1 1] DestroysTheCoinMesh
      (`StaticMeshComponent.SetStaticMesh` _coin null)
      (`KismetSystemLibrary.Delay` 7.0)
      (`StaticMeshComponent.SetStaticMesh` _coin "/Game/Assets/Meshes/SM_Coin.SM_Coin"))
    (:`then_1`
      ;[1 1 1] DisablesCharacterInput
      (bind _outactors (`GameplayStatics.GetAllActorsOfClass` "/Game/Blueprints/MyCharacter.MyCharacter_C"))
      (message `/Game/Assets/Blueprints/BPI_DisableInput.DisableControllerInput` _outactors))
    (:`then_2`
      ;[1 1 1] Waits 3 Seconds to Move The Character To Next Level and Destroys The Actor
      (`KismetSystemLibrary.Delay` 3.0)
      (`|ExecutionSequence`
        (:`then_0`
          (bind _asmy_character (cast `/Game/Blueprints/MyCharacter` (`GameplayStatics.GetPlayerCharacter` 0)))
          (switch `int` (`self.NextLevel`)
            (:`1`
              (`/Game/Blueprints/MyCharacter.MoveToLevel1` _asmy_character))
            (:`2`
              (`/Game/Blueprints/MyCharacter.MoveToLevel2` _asmy_character))
            (:`3`
              (`/Game/Blueprints/MyCharacter.MoveToLevel3` _asmy_character))
            (:`4`
              (`/Game/Blueprints/MyCharacter.MoveToLevel4` _asmy_character))
            (:`5`
              (`/Game/Blueprints/MyCharacter.MoveToLevel5` _asmy_character))
            (:`6`
              (`/Game/Blueprints/MyCharacter.MoveToLevel6` _asmy_character))
            (:`7`
              (`/Game/Blueprints/MyCharacter.MoveToLevel7` _asmy_character))
            (:`8`
              (`/Game/Blueprints/MyCharacter.MoveToLevel8` _asmy_character))
            (:`9`
              (`/Game/Blueprints/MyCharacter.MoveToLevel9` _asmy_character))))))
    (:`then_3`
      ;[1 1 1] Disables The Level Skip Feature And Re-Enables It
      (bind _asmy_character_2 (cast `/Game/Blueprints/MyCharacter` (`GameplayStatics.GetPlayerCharacter` 0)))
      (set `/Game/Blueprints/MyCharacter.bEnableLevelSkip` false _asmy_character_2)
      (`KismetSystemLibrary.Delay` 7.0)
      (set `/Game/Blueprints/MyCharacter.bEnableLevelSkip` true _asmy_character_2))))

(fn `UserConstructionScript`
  (`PrimitiveComponent.SetMaterial` (`self.Coin`) 0 (`self.CoinMaterial`)))