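; Wind vent actor that launches Characters touching its base along its up vector and lifts them through a wind column.
; While WindOverlap's gate is open, Tick forces Falling and adds clamped upward velocity, mapped from player pawn 0's distance to the vent.
; The construction script tiles stretched spiral and plane meshes to the editable Height, fades their materials near the top, and fits the wind box and Papers particle lifetime.
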(event `self.Vent overlap.OnComponentBeginOverlap`
  (params (OtherActor :type "Actor Object Reference") (OtherComp :type "PrimitiveComponent Object Reference") (OtherBodyIndex :type Integer) (bFromSweep :type Boolean) (SweepResult :type "EngineTypes.HitResult Structure (by ref)"))
  ;[1 1 1] Launch character if he hits the bottom of the vent
  (bind _ascharacter (cast `Character` OtherActor))
  (`Character.LaunchCharacter` _ascharacter (* (`KismetMathLibrary.GetUpVector` (`self.K2_GetActorRotation`)) (`self.Boost Amount`)) true true))

(event `self.ReceiveTick`
  (params (DeltaSeconds :type "Float (single-precision)"))
  ;[1 1 1] Push character upwards based on distance to vent
  (`/Engine/EditorBlueprintResources/StandardMacros.Gate` true :!label _label
    (:`Exit`
      (bind _charactermovement (`Character.CharacterMovement` (stale `self.Wind overlap.OnComponentBeginOverlap` _ascharacter)))
      (`CharacterMovementComponent.SetMovementMode` _charactermovement "MOVE_Falling" 0)
      (bind _returnvalue (`self.GetDistanceTo` (`GameplayStatics.GetPlayerPawn` 0)))
      (set `MovementComponent.Velocity` (`KismetMathLibrary.ClampVectorSize` (+ (`MovementComponent.Velocity` _charactermovement) (* (* (`KismetMathLibrary.GetUpVector` (`self.K2_GetActorRotation`)) (* (`KismetMathLibrary.MapRange` _returnvalue 0.0 (`self.Height Z`) (`self.Max Push`) (`self.Min Push`)) 5.0)) (`GameplayStatics.GetWorldDeltaSeconds`))) 0.0 5000.0) _charactermovement))))

(event `self.Wind overlap.OnComponentBeginOverlap`
  (params (OtherActor :type "Actor Object Reference") (OtherComp :type "PrimitiveComponent Object Reference") (OtherBodyIndex :type Integer) (bFromSweep :type Boolean) (SweepResult :type "EngineTypes.HitResult Structure (by ref)"))
  ;[1 1 1] Push character upwards based on distance to vent
  (bind _ascharacter (cast `Character` OtherActor))
  (goto _label :!via `Open`))

(event `self.Wind overlap.OnComponentEndOverlap`
  (params (OtherActor :type "Actor Object Reference") (OtherComp :type "PrimitiveComponent Object Reference") (OtherBodyIndex :type Integer))
  ;[1 1 1] Push character upwards based on distance to vent
  (goto _label :!via `Close`))

(fn `UserConstructionScript`
  (bind _wind_overlap (`self.Wind overlap`))
  (bind _z (.z (`self.Height`)))
  (bind _returnvalue (/ (`self.Height Z`) 2.0))
  (bind _returnvalue_2 (/ (/ (`self.Height Z`) 1000.0) (`self.Max Stretching`)))
  (bind _returnvalue_3 (`KismetMathLibrary.FCeil` _returnvalue_2))
  (bind _returnvalue_4 (`KismetMathLibrary.Conv_IntToDouble` _returnvalue_3))
  (`|ExecutionSequence`
    (:`then_0`
      (set `self.Height` (`KismetMathLibrary.MakeVector` 0.0 0.0 _z))
      (set `self.Height Z` _z)
      (set `self.Piece Scale` (/ (/ (`self.Height Z`) 1000.0) _returnvalue_4))
      (set `self.Number of Pieces` _returnvalue_3)
      (for _index (range (+ (`KismetMathLibrary.FFloor` _returnvalue_2) 1))
        (bind _returnvalue_5 (`KismetMathLibrary.MakeVector` 0.0 0.0 (* (`KismetMathLibrary.Conv_IntToDouble` (* _index 1000)) (/ (/ (`self.Height Z`) 1000.0) _returnvalue_4))))
        (bind _returnvalue_6 (`AddComponent|StaticMeshComponent_28338` :`RelativeTransform` (`KismetMathLibrary.MakeTransform` _returnvalue_5 (struct) (`KismetMathLibrary.MakeVector` 5.0 5.0 (* (`self.Piece Scale`) 5.0)))))
        (`|ExecutionSequence`
          (:`then_0`
            (`/Engine/EditorBlueprintResources/StandardMacros.DoOnce` false
              (:`Completed`
                (set `self.FirstSpiral` _returnvalue_6)
                (`PrimitiveComponent.SetCastShadow` (`self.FirstSpiral`) false))))
          (:`then_2`
            (bind _returnvalue_7 (`AddComponent|StaticMeshComponent_68229` :`RelativeTransform` (`KismetMathLibrary.MakeTransform` _returnvalue_5 (struct) (`KismetMathLibrary.MakeVector` 5.0 -5.0 (* (`self.Piece Scale`) 5.0)))))
            (`|ExecutionSequence`
              (:`then_0`
                (`/Engine/EditorBlueprintResources/StandardMacros.DoOnce` false
                  (:`Completed`
                    (set `self.First Thinspiral` _returnvalue_7)
                    (`PrimitiveComponent.SetCastShadow` (`self.First Thinspiral`) false))))
              (:`then_2`
                (bind _returnvalue_8 (`AddComponent|StaticMeshComponent_68249` :`RelativeTransform` (`KismetMathLibrary.MakeTransform` _returnvalue_5 (struct :`Yaw` 90.0) (`KismetMathLibrary.MakeVector` 20.0 1.0 (* (`self.Piece Scale`) 10.0)))))
                (`|ExecutionSequence`
                  (:`then_0`
                    (`/Engine/EditorBlueprintResources/StandardMacros.DoOnce` false
                      (:`Completed`
                        (set `self.First Plane` _returnvalue_8)
                        (`PrimitiveComponent.SetCastShadow` (`self.First Plane`) false))))
                  (:`then_2`
                    (bind _returnvalue_9 (`PrimitiveComponent.CreateDynamicMaterialInstance` _returnvalue_6 0 null))
                    (bind _returnvalue_10 (`PrimitiveComponent.CreateDynamicMaterialInstance` _returnvalue_7 0 null))
                    (bind _returnvalue_11 (`PrimitiveComponent.CreateDynamicMaterialInstance` _returnvalue_8 0 null))
                    (`MaterialInstanceDynamic.SetScalarParameterValue` _returnvalue_9 "Falloff Begin" (- (.z (`KismetMathLibrary.TransformLocation` (`self.GetTransform`) (- (`self.Height`) (0.0 0.0 100.0)))) 32.0))
                    (`MaterialInstanceDynamic.SetScalarParameterValue` _returnvalue_10 "Falloff Begin" (- (.z (`KismetMathLibrary.TransformLocation` (`self.GetTransform`) (- (`self.Height`) (0.0 0.0 100.0)))) 32.0))
                    (`MaterialInstanceDynamic.SetScalarParameterValue` _returnvalue_11 "Falloff Begin" (- (.z (`KismetMathLibrary.TransformLocation` (`self.GetTransform`) (- (`self.Height`) (0.0 0.0 100.0)))) 32.0))))))))))
    (:`then_1`
      (`BoxComponent.SetBoxExtent` _wind_overlap (`KismetMathLibrary.MakeVector` 200.0 200.0 _returnvalue) true)
      (`SceneComponent.SetRelativeLocation` _wind_overlap (`KismetMathLibrary.MakeVector` 0.0 0.0 _returnvalue) false)
      (`ParticleSystemComponent.SetFloatParameter` (`self.papers`) "lifetime" (/ (`self.Height Z`) 300.0)))))